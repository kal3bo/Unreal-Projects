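; Pickup Blueprint for a camera lid that carries four screws.
; On BeginPlay, after running the parent logic, it attaches the root component of each screw's child actor to the lid's static mesh, keeping world transforms.
; This parenting makes the screws move along with the lid when the user grabs the whole camera.
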(event `self.ReceiveBeginPlay`
  ;[0.9992 0.5194 1] Parenting the screws to the lid in order to move them along when the user grabs the whole camera.
  (`parent.ReceiveBeginPlay`)
  (`|ExecutionSequence`
    (:`then_0`
      (`SceneComponent.K2_AttachToComponent` (`Actor.RootComponent` (`ChildActorComponent.ChildActor` (`self.Screw_1`))) (`self.StaticMeshComponent`) "None" "KeepWorld" "KeepWorld" "KeepWorld" true))
    (:`then_1`
      (`SceneComponent.K2_AttachToComponent` (`Actor.RootComponent` (`ChildActorComponent.ChildActor` (`self.Screw_2`))) (`self.StaticMeshComponent`) "None" "KeepWorld" "KeepWorld" "KeepWorld" true))
    (:`then_2`
      (`SceneComponent.K2_AttachToComponent` (`Actor.RootComponent` (`ChildActorComponent.ChildActor` (`self.Screw_3`))) (`self.StaticMeshComponent`) "None" "KeepWorld" "KeepWorld" "KeepWorld" true))
    (:`then_3`
      (`SceneComponent.K2_AttachToComponent` (`Actor.RootComponent` (`ChildActorComponent.ChildActor` (`self.Screw_4`))) (`self.StaticMeshComponent`) "None" "KeepWorld" "KeepWorld" "KeepWorld" true))))

(fn `UserConstructionScript`
  (`parent.UserConstructionScript`))