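; BP_Pickup_Camera is a camera pickup actor assembled from a camera mesh and child actors for two batteries and a lid.
; On BeginPlay, after calling the parent, it attaches the root component of each battery and the lid to the camera's static mesh with KeepWorld rules, so the parts move along with it.
; The construction script only calls its parent.
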(event `self.ReceiveBeginPlay`
  ;[1 0.4181 0.8475] Parenting the batteries and the lid to the camera in order to move them along with everything.
  (`parent.ReceiveBeginPlay`)
  (`|ExecutionSequence`
    (:`then_0`
      (`SceneComponent.K2_AttachToComponent` (`Actor.RootComponent` (`ChildActorComponent.ChildActor` (`self.Battery_02`))) (`self.StaticMeshComponent`) "None" "KeepWorld" "KeepWorld" "KeepWorld" true))
    (:`then_1`
      (`SceneComponent.K2_AttachToComponent` (`Actor.RootComponent` (`ChildActorComponent.ChildActor` (`self.Battery_01`))) (`self.StaticMeshComponent`) "None" "KeepWorld" "KeepWorld" "KeepWorld" true))
    (:`then_2`
      (`SceneComponent.K2_AttachToComponent` (`Actor.RootComponent` (`ChildActorComponent.ChildActor` (`self.Lid`))) (`self.StaticMeshComponent`) "None" "KeepWorld" "KeepWorld" "KeepWorld" true))))

(fn `UserConstructionScript`
  (`parent.UserConstructionScript`))